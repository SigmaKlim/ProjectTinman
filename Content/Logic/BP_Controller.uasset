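; BP_Controller is a player controller that routes Enhanced Input look and move actions to the player character.
; On BeginPlay it adds the IMC_Default mapping context to the local player's input subsystem.
; On possess it casts the pawn to PT_Protagonist and stores it as ProtagonistPawn.
; The IA_Look and IA_Move handlers forward their X and Y values to PTLook and PTMove on a separately named ControlledPlayer reference.
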(event EventBeginPlay
  (Input|AddMappingContext (PlayerController|LocalPlayerSubsystems|GetEnhancedInputLocalPlayerSubsystem) "/Game/Logic/Input/IMC_Default.IMC_Default" 0 "(bIgnoreAllPressedKeysUntilRelease=True,bForceImmediately=False,bNotifyUserSettings=False)"))

(event EventTick
  (params (DeltaSeconds :type Float%20%28single-precision%29)))

(event EventPossess
  (params (PossessedPawn :type Pawn%20Object%20Reference))
  (bind _aspt_protagonist (Utilities|Casting|CastToPT_Protagonist PossessedPawn))
  (Variables|Default|SetProtagonistPawn _aspt_protagonist))

(event Input|EnhancedActionEvents|EnhancedInputActionIA_Look
  (params (ActionValue :type Vector%202D%20Structure) (ElapsedSeconds :type Float%20%28double-precision%29) (TriggeredSeconds :type Float%20%28double-precision%29) (InputAction :type Input%20Action%20Object%20Reference :default "/Game/Logic/Input/Actions/IA_Look.IA_Look"))
  (bind (_x _y) (Math|Vector2D|BreakVector2D ActionValue))
  (Class|PTProtagonist|PTLook (Variables|Default|GetControlledPlayer) _x _y))

(event Input|EnhancedActionEvents|EnhancedInputActionIA_Move
  (params (ActionValue :type Vector%202D%20Structure) (ElapsedSeconds :type Float%20%28double-precision%29) (TriggeredSeconds :type Float%20%28double-precision%29) (InputAction :type Input%20Action%20Object%20Reference :default "/Game/Logic/Input/Actions/IA_Move.IA_Move"))
  (bind (_x _y) (Math|Vector2D|BreakVector2D ActionValue))
  (Class|PTProtagonist|PTMove (Variables|Default|GetControlledPlayer) _x _y))

(fn ConstructionScript)